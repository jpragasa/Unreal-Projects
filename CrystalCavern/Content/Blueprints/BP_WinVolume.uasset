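; BP_WinVolume is a trigger actor that completes the level when the player overlaps it with no BP_Crystal actors left in the world.
; Completion finds the current level's index in the LevelNames array and opens the following entry by name.
; On the array's last level, it prints a win message and quits the game instead.
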(event Collision|EventActorBeginOverlap
  (params (OtherActor :type Actor%20Object%20Reference))
  (Utilities|IsPlayer OtherActor
    (:IsPlayer
      (if (not (CallFunction|AnyCrystalsRemaining))
        (CallFunction|CompleteLevel)))))

(fn ConstructionScript)

(fn AnyCrystalsRemaining
  (bind _outactors (Actor|GetAllActorsOfClass "/Game/Blueprints/BP_Crystal.BP_Crystal_C"))
  (return (> (Utilities|Array|Length _outactors) 0)))

(fn CompleteLevel
  (if (CallFunction|IsFinalLevel)
    (Development|PrintString "You Win!")
    (Game|QuitGame 0 "Quit" false)
    (else
      (CallFunction|LoadNextLevel))))

(fn GetCurrentLevelIndex
  (bind _returnvalue (Game|GetCurrentLevelName true))
  (return (Utilities|Array|FindItem (Variables|Default|GetLevelNames) (Utilities|String|StringToName _returnvalue))))

(fn IsFinalLevel
  (return (== (CallFunction|GetCurrentLevelIndex) (Utilities|Array|LastIndex (Variables|Default|GetLevelNames)))))

(fn LoadNextLevel
  (Game|OpenLevel(byName) (CallFunction|GetNextLevelName)))

(fn GetNextLevelName
  (bind _result (Math|Integer|IncrementInt (CallFunction|GetCurrentLevelIndex))
    (:%20%20
      (return (Utilities|Array|Get(acopy) (Variables|Default|GetLevelNames) _result)))))