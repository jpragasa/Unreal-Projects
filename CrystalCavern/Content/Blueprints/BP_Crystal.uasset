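; BP_Crystal is a collectible crystal that flies into the player and vanishes when the player overlaps it.
; On overlap it stores its location, scale and point light intensity, then plays CollectionTimeline.
; Three timeline tracks drive lerps that home it on the pawn's current position, shrink it to zero and fade out its light.
; The actor destroys itself when the timeline finishes, without awarding anything itself.
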(event EventBeginPlay)

(event Collision|EventActorBeginOverlap
  (params (OtherActor :type Actor%20Object%20Reference))
  (Utilities|IsPlayer OtherActor
    (:IsPlayer
      (CallFunction|StoreStartingValues)
      (bind (_direction _collectionprogress _scaleprogress _lightintensityprogress) (Timeline|Collection%20Timeline Play)
        (:Update
          (CallFunction|MovetoPlayer _collectionprogress)
          (CallFunction|FadeScale _scaleprogress)
          (CallFunction|AdjustLight _lightintensityprogress))
        (:Finished
          (Actor|DestroyActor))))))

(event EventTick
  (params (DeltaSeconds :type Float%20%28single-precision%29)))

(fn ConstructionScript)

(fn MovetoPlayer
  (params (Alpha :type Float%20%28single-precision%29))
  (Transformation|SetActorLocation (Math|Vector|Lerp(Vector) (Variables|Default|GetStartLocation) (Transformation|GetActorLocation (Game|Player|GetPlayerPawn 0)) Alpha) false false))

(fn StoreStartingValues
  (Variables|Default|SetStartLocation (Transformation|GetActorLocation))
  (Variables|Default|SetStartScale (Transformation|GetActorScale3D))
  (Variables|Default|SetLightIntensity (Variables|/Script/Engine.LightComponentBase|GetIntensity (Variables|Default|GetPointLight))))

(fn FadeScale
  (params (Alpha :type Float%20%28single-precision%29))
  (Transformation|SetActorScale3D (Math|Vector|Lerp(Vector) (Variables|Default|GetStartScale) "0, 0, 0" Alpha)))

(fn AdjustLight
  (params (Alpha :type Float%20%28double-precision%29))
  (Rendering|Components|Light|SetIntensity (Variables|Default|GetPointLight) (Math|Float|Lerp (Variables|Default|GetLightIntensity) 0.0 Alpha)))