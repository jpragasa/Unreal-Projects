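; BP_Cannon is an automatic cannon that repeatedly fires projectiles from the moment play begins.
; Each cycle waits for FireRate, then spawns a projectile at the Arrow component's location and rotation, scaled by ProjectileScale.
; BarrelFireTimeline then slides CannonHead along its local Y axis to animate the shot, and its Cannon Fired event track restarts the cycle, so no Tick or timer is used.
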(event EventBeginPlay
  (Utilities|FlowControl|Delay (Variables|Default|GetFireRate) :!label _label)
  (CallFunction|SpawnProjectile)
  (bind _barreltranslateprogress (Timeline|BarrelFireTimeline PlayFromStart)
    (:Update
      (CallFunction|MoveCannonHead _barreltranslateprogress))
    (:CannonFired
      (goto _label))))

(event Collision|EventActorBeginOverlap
  (params (OtherActor :type Actor%20Object%20Reference)))

(event EventTick
  (params (DeltaSeconds :type Float%20%28single-precision%29)))

(fn ConstructionScript)

(fn SpawnProjectile
  (bind _arrow (Variables|Default|GetArrow))
  (Game|SpawnActorfromClass "/Game/Blueprints/BP_Projectile.BP_Projectile_C" (Math|Transform|MakeTransform (Transformation|GetWorldLocation _arrow) (Transformation|GetWorldRotation _arrow) (Math|Conversions|ToVector(Float) (Variables|Default|GetProjectileScale))) "Undefined" "MultiplyWithRoot" 0 0))

(fn MoveCannonHead
  (params (Alpha :type Float%20%28double-precision%29))
  (Transformation|SetRelativeLocation (Variables|Default|GetCannon%20Head) (Math|Vector|MakeVector 0.0 (Math|Float|Lerp -1.5 0.0 Alpha) 0.0) false false))