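; BP_Alien is an enemy character that chases the player and attacks at close range.
; A BeginPlay loop reissues AI MoveTo while alive; Tick halts movement and plays the attack montage when in range, resuming on completion.
; DamagePlayer applies per-hit damage but is not called within this Blueprint.
; Lethal damage disables movement and collision, increments BP_Marine's kills, registers the death with BP_MMGameMode, then destroys the actor after a delay.
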(event EventBeginPlay
  (if (CallFunction|IsAlive) :!label _label
    (AI|AIMoveTo self "0, 0, 0" (Game|GetPlayerCharacter 0) 5.0 false
      (:then
        _)
      (:OnSuccess
        _)
      (:OnFail
        _))
    (Utilities|FlowControl|Delay (Variables|Default|GetAIStopTime))
    (goto _label)))

(event Collision|EventActorBeginOverlap
  (params (OtherActor :type Actor%20Object%20Reference)))

(event EventTick
  (params (DeltaSeconds :type Float%20%28single-precision%29))
  (if (CallFunction|CanAttack)
    (CallFunction|DeactivateAIMovement)
    (Animation|Montage|PlayMontage (Variables|Character|GetMesh) "/Game/Characters/Enemy_Great_Spider/Animations/AlienAttack.AlienAttack"
      (:OnCompleted
        (CallFunction|ActivateAIMovement)))))

(event Game|Damage|EventAnyDamage
  (params (Damage :type Float%20%28single-precision%29) (DamageType :type Damage%20Type%20Object%20Reference) (InstigatedBy :type Controller%20Object%20Reference) (DamageCauser :type Actor%20Object%20Reference))
  (if (CallFunction|IsAlive)
    (bind _output_get (CallFunction|DecreaseHealth Damage))
    (if (<= _output_get 0.0)
      (CallFunction|KIllAI)
      (Utilities|FlowControl|Delay 3.0)
      (Actor|DestroyActor))))

(fn ConstructionScript)

(fn IsWithinAttackRange
  (return (< (Transformation|GetDistanceTo (Game|GetPlayerCharacter 0) self) (Variables|Default|GetAttackRange))))

(fn IsAttacking
  (return (Animation|Montage|MontageIsPlaying (Components|SkeletalMesh|GetAnimInstance (Variables|Character|GetMesh)) 0)))

(fn DeactivateAIMovement
  (bind _charactermovement (Variables|Character|GetCharacterMovement))
  (Components|Activation|Deactivate _charactermovement)
  (Components|Movement|StopMovementImmediately _charactermovement))

(fn ActivateAIMovement
  (Components|Activation|Activate (Variables|Character|GetCharacterMovement) false))

(fn DamagePlayer
  (if (CallFunction|IsAlive)
    (Game|Damage|ApplyDamage (Game|GetPlayerCharacter 0) (Variables|Default|GetDamagePerHit) 0 0)))

(fn DecreaseHealth
  (params (B :type Float%20%28double-precision%29))
  (bind _output_get (Variables|Default|SetAlienHealth (- (Variables|Default|GetAlienHealth) B)))
  (return _output_get))

(fn KIllAI
  (Variables|Default|SetDead true)
  (CallFunction|DeactivateAIMovement)
  (Collision|SetActorEnableCollision false)
  (bind _asbp_marine (Utilities|Casting|CastToBP_Marine (Game|GetPlayerCharacter 0)))
  (Default|IncreaseKIlls _asbp_marine)
  (bind _asbp_mmgame_mode (Utilities|Casting|CastToBP_MMGameMode (Game|GetGameMode)))
  (Default|RegisterAlienDeath _asbp_mmgame_mode self))

(fn IsAlive
  (return (not (Variables|Default|GetDead))))

(fn CanAttack
  (return (Math|Boolean|ANDBoolean (CallFunction|IsWithinAttackRange) (not (CallFunction|IsAttacking)) (CallFunction|IsAlive))))